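; Projectile is a laser projectile actor that damages non-friendly actors it overlaps.
; On overlap, targets implementing IDamageable without the "Friendly" tag receive the damage through an interface message, with a hit sound and spark emitter, and the projectile destroys itself.
; It passes through friendly damageable actors and is destroyed without effects on overlapping anything non-damageable.
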(event `self.ReceiveActorBeginOverlap`
  (params (OtherActor :type "Actor Object Reference"))
  (bind (_returnvalue_location _returnvalue_rotation) (`KismetMathLibrary.BreakTransform` (`self.GetTransform`)))
  (if (`KismetSystemLibrary.DoesImplementInterface` OtherActor "/Game/Blueprints/iDamageable.iDamageable_C")
    (if (not (`self.ActorHasTag` OtherActor "Friendly"))
      (message `/Game/Blueprints/iDamageable.AffectHealth` OtherActor (`self.Damage`))
      (`GameplayStatics.PlaySoundAtLocation` "/Game/Sound/laser-hit.laser-hit" (`SceneComponent.K2_GetComponentLocation` (`self.DefaultSceneRoot`)) (struct) 2.0)
      (`GameplayStatics.SpawnEmitterAtLocation` "/Game/StarterContent/Particles/LaserSpark.LaserSpark" _returnvalue_location _returnvalue_rotation)
      (`self.K2_DestroyActor` :!label _label))
    (else
      (goto _label))))

(fn `UserConstructionScript`)