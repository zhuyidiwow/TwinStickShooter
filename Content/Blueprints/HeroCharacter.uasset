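; Player hero character for a twin-stick shooter, handling movement, aim-to-fire, health and death.
; BeginPlay spawns a weapon onto the mesh's GunSocket, records the spawn transform in TwinStickMode and adds the HUD.
; Move axes drive world-space movement, while fire axes past a deadzone set control rotation and pull the weapon trigger.
; AffectHealth recalculates health; on death it disables input, waits, requests a GameMode respawn and destroys hero and weapon.
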(event `/Game/Blueprints/iDamageable.AffectHealth`
  (params (Delta :type "Float (single-precision)"))
  ;[1 1 1] Take Damage
  (`self.CalculateHealth` Delta)
  (if (`self.isDead`)
    (`self.DisableInput` null)
    (`KismetSystemLibrary.Delay` 3.0)
    (`/Game/Blueprints/TwinStickMode.RespawnPlayer` (`self.GameMode`))
    (`self.K2_DestroyActor` (`self.Weapon`))
    (`self.K2_DestroyActor` self)))

(event `self.ReceiveBeginPlay`
  (bind _mesh (`self.Mesh`))
  ;[1 1 1] Setup Weapon
  (`|ExecutionSequence`
    (:`then_0`
      (bind _returnvalue (`|SpawnActorFromClass` "/Game/Blueprints/Weapon.Weapon_C" (`SceneComponent.K2_GetComponentToWorld` _mesh) "Undefined" "OverrideRootScale" null null))
      (bind _output_get (set `self.Weapon` _returnvalue))
      (`self.K2_AttachToComponent` _output_get _mesh "GunSocket" "SnapToTarget" "SnapToTarget" "KeepWorld" true))
    (:`then_1`
      (bind _astwin_stick_mode (cast `/Game/Blueprints/TwinStickMode` (`GameplayStatics.GetGameMode`)))
      (bind _output_get_2 (set `self.GameMode` _astwin_stick_mode))
      (set `/Game/Blueprints/TwinStickMode.PlayerSpawnTransform` (`self.GetTransform`) _output_get_2))
    (:`then_2`
      (bind _returnvalue_2 (`|CreateWidget` "/Game/Blueprints/TwinStickHUD.TwinStickHUD_C"))
      (`UserWidget.AddToViewport` _returnvalue_2 0))))

(event `InputAxis|MoveUp`
  (params (AxisValue :type "Float (single-precision)"))
  ;[1 1 1] Movement
  (`self.AddMovementInput` (1.0 0.0 0.0) AxisValue))

(event `InputAxis|FireUp`
  (params (AxisValue :type "Float (single-precision)"))
  (bind _weapon (`self.Weapon`))
  ;[1 1 1] Rotation
  (bind _returnvalue (`KismetMathLibrary.MakeVector` AxisValue (stale `InputAxis|FireRight` AxisValue)))
  (if (> (`KismetMathLibrary.VSize` _returnvalue) 0.25) :!label _label
    (`Controller.SetControlRotation` (`self.GetController`) (`KismetMathLibrary.Conv_VectorToRotator` _returnvalue))
    (`/Game/Blueprints/Weapon.PullTrigger` _weapon)
    (else
      (`/Game/Blueprints/Weapon.ReleaseTrigger` _weapon))))

(event `InputAxis|FireRight`
  (params (AxisValue :type "Float (single-precision)"))
  ;[1 1 1] Rotation
  (goto _label))

(event `InputAxis|MoveRight`
  (params (AxisValue :type "Float (single-precision)"))
  ;[1 1 1] Movement
  (`self.AddMovementInput` (0.0 1.0 0.0) AxisValue))

(fn `UserConstructionScript`)