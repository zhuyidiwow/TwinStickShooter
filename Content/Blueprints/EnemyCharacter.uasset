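; Enemy character Blueprint that takes damage, hurts the hero on contact and is tinted by its EnemyColor.
; AffectHealth recalculates health and destroys the actor once IsDead is set.
; Overlapping a HeroCharacter stores it and starts a looping timer that applies Damage through the hero's AffectHealth, cleared by function name when that overlap ends.
; The construction script applies the color through a dynamic material instance.
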(event `/Game/Blueprints/iDamageable.AffectHealth`
  (params (Delta :type "Float (single-precision)"))
  ;[1 1 1] Take Damage
  (`self.CalculateHealth` Delta)
  (`KismetSystemLibrary.PrintString` (`KismetStringLibrary.Conv_DoubleToString` (`self.Health`)))
  (if (`self.isDead`)
    (`self.K2_DestroyActor`)))

(event `self.ReceiveActorBeginOverlap`
  (params (OtherActor :type "Actor Object Reference"))
  ;[1 1 1] Damage Player
  (bind _ashero_character (cast `/Game/Blueprints/HeroCharacter` OtherActor))
  (set `self.Hero` _ashero_character)
  (`KismetSystemLibrary.K2_SetTimerDelegate` (delegate `DamageTheHero`) 0.5 true))

(event `DamageTheHero`
  ;[1 1 1] Damage Player
  (`/Game/Blueprints/HeroCharacter.AffectHealth` (`self.Hero`) (`self.Damage`))
  (`KismetSystemLibrary.PrintString` (`KismetStringLibrary.Conv_DoubleToString` (`BaseCharacter.Health` (`self.Hero`)))))

(event `self.ReceiveActorEndOverlap`
  (params (OtherActor :type "Actor Object Reference"))
  (if (== OtherActor (`self.Hero`))
    (`KismetSystemLibrary.K2_ClearTimer` null "DamageTheHero")))

(fn `UserConstructionScript`
  (bind _returnvalue (`PrimitiveComponent.CreateDynamicMaterialInstance` (`self.Mesh`) 0 null))
  (bind _output_get (set `self.DynaMat` _returnvalue))
  (`MaterialInstanceDynamic.SetVectorParameterValue` _output_get "BodyColor" (`self.EnemyColor`)))